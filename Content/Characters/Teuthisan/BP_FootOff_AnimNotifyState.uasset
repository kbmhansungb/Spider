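; Anim notify state for the Teuthisan character that tracks a foot-off window in an animation for one named socket.
; Each tick it calls UpdateBonePosition on that socket.
; On end it gets the foot-off data object from the AnimInstance through ReactToFeetOffInterface and rewrites the socket's map entry, clearing one flag while keeping positions and hit state.
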(fn `Received_NotifyEnd`
  (params (MeshComp :type "SkeletalMeshComponent Object Reference") (Animation :type "AnimSequenceBase Object Reference") (EventReference :type "AnimNotifyEventReference Structure (by ref)"))
  (returns (ReturnValue :type Boolean))
  (bind _socketname (`self.SocketName`))
  (bind _asreact_to_feet_off_interface (cast `ReactToFeetOffInterface` (`SkeletalMeshComponent.GetAnimInstance` MeshComp)))
  (bind _returnvalue (`ReactToFeetOffInterface.GetFootOfDataObject` _asreact_to_feet_off_interface))
  (bind _footofdatamap (`FootOffDataObject.FootOfDataMap` _returnvalue))
  (bind _value (`BlueprintMapLibrary.Map_Find` _footofdatamap _socketname))
  (`BlueprintMapLibrary.Map_Add` _footofdatamap _socketname (make `FootOfData` (break `FootOfData` _value) (`.HitPosition` (break `FootOfData` _value)) false (`.IsHit` (break `FootOfData` _value))))
  (return false))

(fn `Received_NotifyTick`
  (params (MeshComp :type "SkeletalMeshComponent Object Reference") (Animation :type "AnimSequenceBase Object Reference") (FrameDeltaTime :type "Float (single-precision)") (EventReference :type "AnimNotifyEventReference Structure (by ref)"))
  (returns (ReturnValue :type Boolean))
  (`self.UpdateBonePosition` MeshComp (`self.SocketName`))
  (return true))